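; Gem pickup Blueprint that plays a short collect animation and then removes itself, with no score or inventory logic.
; The first overlap by any actor sets Collected and starts a one-second DeathTimer that destroys the actor.
; Tick constantly spins the gem and, once collected, moves it vertically by a steadily decreasing LiftSpeed while shrinking it.
; All motion uses fixed per-frame steps, so it is frame-rate dependent.
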(event `self.ReceiveActorBeginOverlap`
  (params (OtherActor :type "Actor Object Reference"))
  (if (not (`self.Collected`))
    (set `self.Collected` true)
    (`KismetSystemLibrary.K2_SetTimer` null "DeathTimer" 1.0)))

(event `self.ReceiveTick`
  (params (DeltaSeconds :type "Float (single-precision)"))
  (bind _liftspeed (`self.LiftSpeed`))
  (`SceneComponent.K2_AddLocalRotation` (`self.Gem`) (struct :`Yaw` 1.0) false false)
  (if (`self.Collected`)
    (`self.K2_AddActorLocalOffset` (`KismetMathLibrary.MakeVector` 0.0 0.0 _liftspeed))
    (set `self.LiftSpeed` (- _liftspeed 0.1))
    (bind _output_get (set `self.Scale` (- (`self.Scale`) (0.01 0.01 0.01))))
    (`self.SetActorScale3D` _output_get)))

(fn `DeathTimer`
  (`self.K2_DestroyActor`))

(fn `UserConstructionScript`)